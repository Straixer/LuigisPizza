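; BP_MotoPrototype is a VR-drivable vehicle prototype that the player steers with a grabbable wheel and drives with a lever.
; Grabbing its grab component toggles boarding, aligning the XR pawn's camera to HeadPosition and attaching VROrigin, or detaching it at ExitPosition.
; Looping timers make held controls follow the motion controller via dot products, setting throttle, brake and steering.
; Tick turns these into clamped speed, yaw and swept movement, without physics.
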(event `self.ReceiveTick`
  (params (DeltaSeconds :type "Float (single-precision)"))
  ;[0 0 0 0.5] Velocidad
  (set `self.CurrentSpeed` (`KismetMathLibrary.FClamp` (+ (* (* (- (`self.Throttle`) (`self.Brake`)) (`self.Acceleration`)) DeltaSeconds) (`self.CurrentSpeed`)) (* (`self.MaxReverseSpeed`) -1.0) (`self.MaxForwardSpeed`)))
  ;[0 0 0 0.5] Aplicación del giro
  (`self.K2_AddActorWorldRotation` (`KismetMathLibrary.MakeRotator` 0.0 0.0 (* (* (`self.SteeringValue`) (`self.TurnSpeed`)) DeltaSeconds)))
  (`self.K2_AddActorWorldOffset` (* (* (`self.GetActorForwardVector`) (`self.CurrentSpeed`)) DeltaSeconds) true))

(event `self.BP_GrabComponent.OnGrabbed`
  (params (`Motion Controller` :type "MotionControllerComponent Object Reference"))
  (bind (_returnvalue_x _returnvalue_y) (`KismetMathLibrary.BreakVector` (`SceneComponent.K2_GetComponentLocation` (`self.ExitPosition`))))
  ;[0 0 0 0.5] Entrada al vehículo
  (bind _asbp_xrpawn (cast `/Game/XRFramework/Blueprints/BP_XRPawn` (`GameplayStatics.GetPlayerPawn` 0)))
  (if (`self.inVehicle?`)
    (bind _vrorigin (`/Game/XRFramework/Blueprints/BP_XRPawn.VROrigin` _asbp_xrpawn))
    (`SceneComponent.K2_SetWorldLocation` _vrorigin (`KismetMathLibrary.MakeVector` _returnvalue_x _returnvalue_y) false false)
    (`HeadMountedDisplayFunctionLibrary.SetTrackingOrigin` "Stage")
    (set `self.inVehicle?` false)
    (`SceneComponent.K2_DetachFromComponent` _vrorigin "KeepWorld" "KeepWorld" "KeepWorld" true)
    (else
      (`SceneComponent.K2_AddWorldOffset` _vrorigin (- (`SceneComponent.K2_GetComponentLocation` (`self.HeadPosition`)) (`SceneComponent.K2_GetComponentLocation` (`/Game/XRFramework/Blueprints/BP_XRPawn.Camera` _asbp_xrpawn))) false false)
      (set `self.inVehicle?` true)
      (`SceneComponent.K2_AttachToComponent` _vrorigin (`self.HeadPosition`) "None" "KeepWorld" "KeepWorld" "KeepWorld" true))))

(event `self.LeverGC.OnGrabbed`
  (params (`Motion Controller` :type "MotionControllerComponent Object Reference"))
  ;[0 0 0 0.5] Palanca
  (set `self.HandleMC` `Motion Controller`)
  (`KismetSystemLibrary.K2_SetTimerDelegate` (delegate `MoveHandle`) 0.01 true))

(event `MoveHandle`
  (bind _handle (`self.Handle`))
  (bind _handle_2 (`self.Handle`))
  (bind (_relativerotation_roll _relativerotation_pitch _relativerotation_yaw) (`KismetMathLibrary.BreakRotator` (`SceneComponent.RelativeRotation` _handle_2)))
  (bind _returnvalue (`KismetMathLibrary.FClamp` (+ _relativerotation_pitch (* (`KismetMathLibrary.Dot_VectorVector` (`KismetMathLibrary.Conv_RotatorToVector` (`KismetMathLibrary.FindLookAtRotation` (`SceneComponent.K2_GetComponentLocation` _handle) (`SceneComponent.K2_GetComponentLocation` (`self.HandleMC`)))) (* (`KismetMathLibrary.GetForwardVector` (`SceneComponent.K2_GetComponentRotation` _handle)) -1.0)) 10.0)) -70.0 70.0))
  (bind _returnvalue_2 (`KismetMathLibrary.MapRangeClamped` _returnvalue -70.0 70.0 1.0 -1.0))
  ;[0 0 0 0.5] Palanca
  (`SceneComponent.K2_SetRelativeRotation` _handle_2 (`KismetMathLibrary.MakeRotator` _relativerotation_roll _returnvalue _relativerotation_yaw) false false)
  (if (>= _returnvalue_2 0.0)
    (set `self.Throttle` _returnvalue_2)
    (set `self.Brake` 0.0)
    (else
      (set `self.Brake` (* _returnvalue_2 -1.0))
      (set `self.Throttle` 0.0))))

(event `self.LeverGC.OnDropped`
  ;[0 0 0 0.5] Palanca
  (`KismetSystemLibrary.K2_PauseTimer` null "MoveHandle"))

(event `self.SteeringGC.OnGrabbed`
  (params (`Motion Controller` :type "MotionControllerComponent Object Reference"))
  ;[0 0 0 0.5] Volante
  (set `self.SteeringMC` `Motion Controller`)
  (`KismetSystemLibrary.K2_SetTimerDelegate` (delegate `RotateWheel`) 0.01 true))

(event `RotateWheel`
  (bind _steeringwheel (`self.SteeringWheel`))
  (bind _steeringwheel_2 (`self.SteeringWheel`))
  (bind _relativerotation_roll (`KismetMathLibrary.BreakRotator` (`SceneComponent.RelativeRotation` _steeringwheel_2)))
  ;[0 0 0 0.5] Volante
  (`SceneComponent.K2_AddLocalRotation` _steeringwheel_2 (`KismetMathLibrary.MakeRotator` (* (`KismetMathLibrary.NormalizeAxis` (`KismetMathLibrary.Dot_VectorVector` (`KismetMathLibrary.Conv_RotatorToVector` (`KismetMathLibrary.FindLookAtRotation` (`SceneComponent.K2_GetComponentLocation` _steeringwheel) (`SceneComponent.K2_GetComponentLocation` (`self.SteeringMC`)))) (`KismetMathLibrary.GetRightVector` (`SceneComponent.K2_GetComponentRotation` _steeringwheel)))) 50.0)) false false)
  (set `self.SteeringValue` (`KismetMathLibrary.MapRangeClamped` _relativerotation_roll 90.0 -90.0 -1.0 1.0)))

(event `self.SteeringGC.OnDropped`
  ;[0 0 0 0.5] Volante
  (`KismetSystemLibrary.K2_PauseTimer` null "RotateWheel")
  (set `self.SteeringMC` null))

(fn `UserConstructionScript`)